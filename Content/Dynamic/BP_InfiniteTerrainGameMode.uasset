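; Game mode for an endless terrain game that builds the level from chained BP_Tile actors.
; On BeginPlay it fills a pool of nav mesh bounds volumes, then spawns the first few tiles in a loop.
; Each new tile receives the pool and returns its attach point, which becomes the transform for the next tile.
; NewTileConquered increments the score and prints it.
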(event `self.ReceiveBeginPlay`
  (`self.PopulateBoundsVolumePool`)
  (for _ (range 4)
    (`self.Spawn Tile`)))

(fn `New Tile Conquered`
  (bind _result (`/Engine/EditorBlueprintResources/StandardMacros.IncrementInt` (`self.Score`))
    (:`  `
      (`KismetSystemLibrary.PrintString` (`KismetStringLibrary.Conv_IntToString` _result)))))

(fn `Spawn Tile`
  (bind _returnvalue (`|SpawnActorFromClass` "/Game/Dynamic/Terrain/BP_Tile.BP_Tile_C" (`self.Next TIle Transform`) "Undefined" "OverrideRootScale" null null))
  (`Tile.SetPool` _returnvalue (`self.NavMeshBoundsVolumePool`))
  (bind _attach_transform (`/Game/Dynamic/Terrain/BP_Tile.Get Attach Location` _returnvalue))
  (set `self.Next TIle Transform` _attach_transform))

(fn `UserConstructionScript`)